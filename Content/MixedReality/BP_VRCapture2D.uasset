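; Scene capture actor for mixed reality that can act as a handheld VR camera tracked by a motion controller.
; It registers the capture component's render target on BeginPlay and removes it when destroyed.
; With FollowController enabled and valid tracking, Tick composes the left-hand pose with the player view target's transform to place the actor in world space.
; A debug cone draw for the controller pose is left unconnected.
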(event EventTick
  (params (DeltaSeconds :type Float%20%28single-precision%29))
  (bind _returnvalue (Game|GetPlayerController 0))
  (bind (_outposition _outorientation _returnvalue_2) (Class|SteamVRFunctionLibrary|GetHandPositionandOrientation 1 "Left"))
  (bind _returnvalue_3 (Pawn|GetViewTarget _returnvalue))
  (bind _returnvalue_4 (Math|Transform|MakeTransform _outposition _outorientation))
  (bind _returnvalue_5 (Transformation|GetActorTransform _returnvalue_3))
  (bind _returnvalue_6 (Math|Transform|ComposeTransforms _returnvalue_4 _returnvalue_5))
  (bind (_location _rotation) (Math|Transform|BreakTransform _returnvalue_6))
  (if (and (Variables|Default|GetFollowController) _returnvalue_2)
    (Transformation|SetActorLocationAndRotation _location _rotation)))

(event EventBeginPlay
  (|CallParentFunction)
  (Class|SteamVRFunctionLibrary|SetCaptureRenderTarget (Variables|/Script/Engine.SceneCaptureComponent2D|GetTextureTarget (Variables|DecalActor|GetCaptureComponent2D))))

(event EventDestroyed
  (|CallParentFunction)
  (Class|SteamVRFunctionLibrary|RemoveCaptureRenderTarget (Variables|/Script/Engine.SceneCaptureComponent2D|GetTextureTarget (Variables|DecalActor|GetCaptureComponent2D))))

(fn ConstructionScript)